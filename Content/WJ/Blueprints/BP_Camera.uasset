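; BP_Camera is a camera actor that smoothly follows BP_Player.
; On BeginPlay it finds the player and stores its initial world offset from them, so the placed position sets the framing.
; Each tick it lerps its location toward the player's location plus that offset, with delta time times Smooth as the alpha; rotation is left untouched.
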(event EventBeginPlay
  (bind _returnvalue (Actor|GetActorOfClass "/Game/UK/Blueprints/BP_Player.BP_Player_C"))
  (bind _output_get (Variables|Default|SetPlayer _returnvalue))
  (Variables|Default|Setoffset (- (Transformation|GetActorLocation) (Transformation|GetActorLocation _output_get))))

(event EventTick
  (params (DeltaSeconds :type Float%20%28single-precision%29))
  (Transformation|SetActorLocation (Math|Vector|Lerp(Vector) (Transformation|GetActorLocation) (+ (Transformation|GetActorLocation (Variables|Default|GetPlayer)) (Variables|Default|Getoffset)) (* DeltaSeconds (Variables|Default|Getsmooth))) false false))

(fn ConstructionScript)